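; Terrain tile for an endless-runner style level that chains onto others through an arrow attach transform.
; Player overlap with the unlock box opens the exit barrier and turns it green.
; Leaving that box relocks it in red and asks InfiniteTerrainGameMode to spawn another tile.
; When the player leaves the destroy box, the tile destroys itself.
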(event `self.UnlockCollisionBox.OnComponentBeginOverlap`
  (params (OverlappedComponent :type "PrimitiveComponent Object Reference") (OtherActor :type "Actor Object Reference") (OtherComp :type "PrimitiveComponent Object Reference") (OtherBodyIndex :type Integer) (bFromSweep :type Boolean) (SweepResult :type "HitResult Structure (by ref)"))
  (`self.IsPlayer` OtherActor)
  (`self.Unlock`))

(event `self.UnlockCollisionBox.OnComponentEndOverlap`
  (params (OverlappedComponent :type "PrimitiveComponent Object Reference") (OtherActor :type "Actor Object Reference") (OtherComp :type "PrimitiveComponent Object Reference") (OtherBodyIndex :type Integer))
  (`self.IsPlayer` OtherActor)
  (`self.Lock`))

(event `self.DestroyCollisionBox.OnComponentEndOverlap`
  (params (OverlappedComponent :type "PrimitiveComponent Object Reference") (OtherActor :type "Actor Object Reference") (OtherComp :type "PrimitiveComponent Object Reference") (OtherBodyIndex :type Integer))
  (`self.IsPlayer` OtherActor)
  (`self.K2_DestroyActor`))

(fn `Get Attach Transform`
  (returns (`Attach Transform` :type "Transform Structure"))
  (return (`SceneComponent.K2_GetComponentToWorld` (`self.Arrow`))))

(fn `Lock`
  (`PrimitiveComponent.SetCollisionEnabled` (`self.ExitBarrier`) "QueryAndPhysics")
  (`PrimitiveComponent.SetMaterial` (`self.ExitBarrier`) 0 "/Game/Dynamic/Terrain/RedBarrierMaterial.RedBarrierMaterial")
  (bind _asinfinite_terrain_game_mode (cast `/Game/Dynamic/InfiniteTerrainGameMode` (`GameplayStatics.GetGameMode`)))
  (`/Game/Dynamic/InfiniteTerrainGameMode.SpawnTile` _asinfinite_terrain_game_mode))

(fn `Unlock`
  (`PrimitiveComponent.SetCollisionEnabled` (`self.ExitBarrier`) "NoCollision")
  (`PrimitiveComponent.SetMaterial` (`self.ExitBarrier`) 0 "/Game/Dynamic/Terrain/GreenBarrierMaterial.GreenBarrierMaterial"))

(fn `UserConstructionScript`)
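; Terrain tile for an infinite-terrain game that scatters containers, junk, sacks and rocks on BeginPlay and takes the game mode's nav mesh bounds volume pool.
; The player's overlap with UnlockCollisionBox toggles the exit barrier between green passable and red blocking.
; When the player leaves DestroyCollisionBox, the tile destroys itself and asks the game mode to spawn another.
; An Arrow supplies the attach transform; AI pawn placement is present but unwired.
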(event `self.UnlockCollisionBox.OnComponentBeginOverlap`
  (params (OverlappedComponent :type "PrimitiveComponent Object Reference") (OtherActor :type "Actor Object Reference") (OtherComp :type "PrimitiveComponent Object Reference") (OtherBodyIndex :type Integer) (bFromSweep :type Boolean) (SweepResult :type "HitResult Structure (by ref)"))
  (`self.IsPlayer` OtherActor)
  (`self.Unlock`))

(event `self.UnlockCollisionBox.OnComponentEndOverlap`
  (params (OverlappedComponent :type "PrimitiveComponent Object Reference") (OtherActor :type "Actor Object Reference") (OtherComp :type "PrimitiveComponent Object Reference") (OtherBodyIndex :type Integer))
  (`self.IsPlayer` OtherActor)
  (`self.Lock`))

(event `self.DestroyCollisionBox.OnComponentEndOverlap`
  (params (OverlappedComponent :type "PrimitiveComponent Object Reference") (OtherActor :type "Actor Object Reference") (OtherComp :type "PrimitiveComponent Object Reference") (OtherBodyIndex :type Integer))
  (`self.IsPlayer` OtherActor)
  (`self.K2_DestroyActor`)
  (bind _asbp_infinite_terrain_game_mode (cast `/Game/Dynamic/BP_InfiniteTerrainGameMode` (`GameplayStatics.GetGameMode`)))
  (`/Game/Dynamic/BP_InfiniteTerrainGameMode.SpawnTile` _asbp_infinite_terrain_game_mode))

(event `self.ReceiveBeginPlay`
  (`self.SpawnActors`)
  (bind _asbp_infinite_terrain_game_mode (cast `/Game/Dynamic/BP_InfiniteTerrainGameMode` (`GameplayStatics.GetGameMode`)))
  (bind _returnvalue (`InfiniteTerrainGameMode.GetNavMeshBoundsVolumePool` _asbp_infinite_terrain_game_mode))
  (`self.SetPool` _returnvalue))

(fn `Get Attach Transform`
  (returns (`Attach Transform` :type "Transform Structure"))
  (return (`SceneComponent.K2_GetComponentToWorld` (`self.Arrow`))))

(fn `Lock`
  (`PrimitiveComponent.SetCollisionResponseToChannel` (`self.ExitBarrier`) "ECC_Pawn" "ECR_Block")
  (`PrimitiveComponent.SetMaterial` (`self.ExitBarrier`) 0 "/Game/Dynamic/Terrain/MI_Barrier_Red.MI_Barrier_Red"))

(fn `SpawnActors`
  (bind _spawnparameters (make `SpawnParameters` 0 2 250.0 1.0 2.0))
  (`self.PlaceActor` "/Game/Dynamic/Terrain/BP_Container.BP_Container_C" (make `SpawnParameters` 1 2 450.0))
  (`self.PlaceActor` "/Game/Dynamic/Terrain/BP_Junk.BP_Junk_C" (make `SpawnParameters` 2 4 150.0 1.0 2.0))
  (`self.PlaceActor` "/Game/Dynamic/Terrain/BP_Sacks.BP_Sacks_C" (make `SpawnParameters` 1 2 200.0 1.0 2.0))
  (`self.PlaceActor` "/Game/Dynamic/Terrain/BP_Rock1.BP_Rock1_C" _spawnparameters)
  (`self.PlaceActor` "/Game/Dynamic/Terrain/BP_Rock2.BP_Rock2_C" _spawnparameters)
  (`self.PlaceActor` "/Game/Dynamic/Terrain/BP_Rock3.BP_Rock3_C" _spawnparameters))

(fn `Unlock`
  (`PrimitiveComponent.SetCollisionResponseToChannel` (`self.ExitBarrier`) "ECC_Pawn" "ECR_Ignore")
  (`PrimitiveComponent.SetMaterial` (`self.ExitBarrier`) 0 "/Game/Dynamic/Terrain/MI_Barrier_Green.MI_Barrier_Green"))

(fn `UserConstructionScript`)
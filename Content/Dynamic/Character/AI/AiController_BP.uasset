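; AI controller for guard characters that runs a patrol and player-detection behavior tree.
; On BeginPlay it sets up the PatrolData blackboard, starts GuardBehaviour and caches the possessed BP_Character as PatrollingGuard.
; Perception updates write actors tagged Player to the PlayerActor blackboard key when sensed, and clear the key and focus when lost, with debug prints on both.
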(event `self.ReceiveBeginPlay`
  (bind _blackboardcomponent (`self.UseBlackboard` "/Game/Dynamic/Character/AI/PatrolData.PatrolData"))
  (set `self.BlackboardComp` _blackboardcomponent)
  (`self.RunBehaviorTree` "/Game/Dynamic/Character/AI/GuardBehaviour.GuardBehaviour")
  (bind _asbp_character (cast `/Game/Dynamic/Character/Behaviour/BP_Character` (`self.K2_GetPawn`)))
  (set `self.PatrollingGuard` _asbp_character))

(event `self.AIPerception.OnTargetPerceptionUpdated`
  (params (Actor :type "Actor Object Reference") (Stimulus :type "AIStimulus Structure"))
  (`self.Update Blackboard Player Key` Actor Stimulus Actor))

(fn `Update Blackboard Player Key`
  (params (ObjectValue :type "Object Object Reference") (AIStimulus :type "AIStimulus Structure (by ref)") (self2 :type "Actor Object Reference"))
  (bind _playeractor (`self.PlayerActor`))
  (bind _blackboardcomp (`self.BlackboardComp`))
  (if (`self.ActorHasTag` self2 "Player")
    (if (`.bSuccessfullySensed` (break `AIStimulus` AIStimulus))
      (`BlackboardComponent.SetValueAsObject` _blackboardcomp _playeractor ObjectValue)
      (`KismetSystemLibrary.PrintString` "yes")
      (else
        (`BlackboardComponent.ClearValue` _blackboardcomp _playeractor)
        (`KismetSystemLibrary.PrintString` "not")
        (`self.K2_ClearFocus`)))))

(fn `UserConstructionScript`)
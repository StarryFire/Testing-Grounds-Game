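; NPC_AI_BP is an AI controller for guard NPCs that tracks the player through perception.
; On BeginPlay it sets up the PatrolData blackboard and runs the GuardBehaviour behavior tree.
; Perception updates write any sensed actor tagged Player to the PlayerActor blackboard key and clear the key when that actor is no longer sensed.
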(event `self.ReceiveBeginPlay`
  (bind _blackboardcomponent (`self.UseBlackboard` "/Game/Dynamic/NPC/AI/PatrolData.PatrolData"))
  (set `self.BlackboardComp` _blackboardcomponent)
  (`self.RunBehaviorTree` "/Game/Dynamic/NPC/AI/GuardBehaviour.GuardBehaviour"))

(event `self.AIPerception.OnTargetPerceptionUpdated`
  (params (Actor :type "Actor Object Reference") (Stimulus :type "AIStimulus Structure"))
  (bind _playeractor (`self.PlayerActor`))
  (bind _blackboardcomp (`self.BlackboardComp`))
  (if (`self.ActorHasTag` Actor "Player")
    (if (`.bSuccessfullySensed` (break `AIStimulus` Stimulus))
      (`BlackboardComponent.SetValueAsObject` _blackboardcomp _playeractor Actor)
      (else
        (`BlackboardComponent.ClearValue` _blackboardcomp _playeractor)))))

(fn `UserConstructionScript`)